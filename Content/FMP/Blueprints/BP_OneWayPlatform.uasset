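; One-way platform actor that players can pass through until they enter its trigger volume, then stand on.
; The Cube ignores the Pawn channel by default.
; When the player character overlaps the Collision component, the Cube switches to blocking Pawns after a short delay, and ending the overlap returns it to ignoring them.
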(event `self.ReceiveBeginPlay`
  ;[1 1 1] One way Platform
  (`PrimitiveComponent.SetCollisionResponseToChannel` (`self.Cube`) "ECC_Pawn" "ECR_Ignore"))

(event `self.collision.OnComponentBeginOverlap`
  (params (OverlappedComponent :type "PrimitiveComponent Object Reference") (OtherActor :type "Actor Object Reference") (OtherComp :type "PrimitiveComponent Object Reference") (OtherBodyIndex :type Integer) (bFromSweep :type Boolean) (SweepResult :type "HitResult Structure (by ref)"))
  ;[1 1 1] One way Platform
  (if (== OtherActor (`GameplayStatics.GetPlayerCharacter` 0))
    (if true
      (`KismetSystemLibrary.Delay` 0.2)
      (`PrimitiveComponent.SetCollisionResponseToChannel` (`self.Cube`) "ECC_Pawn" "ECR_Block"))))

(event `self.collision.OnComponentEndOverlap`
  (params (OverlappedComponent :type "PrimitiveComponent Object Reference") (OtherActor :type "Actor Object Reference") (OtherComp :type "PrimitiveComponent Object Reference") (OtherBodyIndex :type Integer))
  ;[1 1 1] One way Platform
  (if (== OtherActor (`GameplayStatics.GetPlayerCharacter` 0))
    (`PrimitiveComponent.SetCollisionResponseToChannel` (`self.Cube`) "ECC_Pawn" "ECR_Ignore")))

(fn `UserConstructionScript`)