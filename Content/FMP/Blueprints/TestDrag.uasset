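; TestDrag is a draggable block actor that slides along its local X axis while BP_Seedboy drags it.
; Overlap hitboxes flag player proximity and side, though RightOfBlock is never cleared.
; Tick moves the block in the player's facing direction at a frame-rate-independent speed while nearby and dragging.
; A second pass handles pulling away from either side, stopping the player's movement and adding another offset.
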(event `self.LeftHitbox.OnComponentBeginOverlap`
  (params (OverlappedComponent :type "PrimitiveComponent Object Reference") (OtherActor :type "Actor Object Reference") (OtherComp :type "PrimitiveComponent Object Reference") (OtherBodyIndex :type Integer) (bFromSweep :type Boolean) (SweepResult :type "HitResult Structure (by ref)"))
  ;[1 1 1] Checks if left or right of block
  ;;[1 1 1] Left of block
  (cast `/Game/FMP/Blueprints/BP_Seedboy` OtherActor)
  (set `self.leftOfBlock` true))

(event `self.RIghtHitbox.OnComponentBeginOverlap`
  (params (OverlappedComponent :type "PrimitiveComponent Object Reference") (OtherActor :type "Actor Object Reference") (OtherComp :type "PrimitiveComponent Object Reference") (OtherBodyIndex :type Integer) (bFromSweep :type Boolean) (SweepResult :type "HitResult Structure (by ref)"))
  ;[1 1 1] Checks if left or right of block
  ;;[1 1 1] Right of block
  (cast `/Game/FMP/Blueprints/BP_Seedboy` OtherActor)
  (set `self.rightOfBlock` true))

(event `self.DragHitbox.OnComponentBeginOverlap`
  (params (OverlappedComponent :type "PrimitiveComponent Object Reference") (OtherActor :type "Actor Object Reference") (OtherComp :type "PrimitiveComponent Object Reference") (OtherBodyIndex :type Integer) (bFromSweep :type Boolean) (SweepResult :type "HitResult Structure (by ref)"))
  ;[1 1 1] If player is near block
  ;;[1 1 1] Toggle
  (cast `/Game/FMP/Blueprints/BP_Seedboy` OtherActor)
  (set `self.inHitbox` true))

(event `self.RIghtHitbox.OnComponentEndOverlap`
  (params (OverlappedComponent :type "PrimitiveComponent Object Reference") (OtherActor :type "Actor Object Reference") (OtherComp :type "PrimitiveComponent Object Reference") (OtherBodyIndex :type Integer))
  ;[1 1 1] Checks if left or right of block
  ;;[1 1 1] Right of block
  (cast `/Game/FMP/Blueprints/BP_Seedboy` OtherActor)
  (set `self.rightOfBlock` true))

(event `self.LeftHitbox.OnComponentEndOverlap`
  (params (OverlappedComponent :type "PrimitiveComponent Object Reference") (OtherActor :type "Actor Object Reference") (OtherComp :type "PrimitiveComponent Object Reference") (OtherBodyIndex :type Integer))
  ;[1 1 1] Checks if left or right of block
  ;;[1 1 1] Left of block
  (cast `/Game/FMP/Blueprints/BP_Seedboy` OtherActor)
  (set `self.leftOfBlock` false))

(event `self.DragHitbox.OnComponentEndOverlap`
  (params (OverlappedComponent :type "PrimitiveComponent Object Reference") (OtherActor :type "Actor Object Reference") (OtherComp :type "PrimitiveComponent Object Reference") (OtherBodyIndex :type Integer))
  ;[1 1 1] If player is near block
  ;;[1 1 1] UnToggle
  (cast `/Game/FMP/Blueprints/BP_Seedboy` OtherActor)
  (set `self.inHitbox` false))

(event `self.ReceiveTick`
  (params (DeltaSeconds :type "Float (single-precision)"))
  (bind _returnvalue (`KismetMathLibrary.Conv_DoubleToVector` DeltaSeconds))
  (`|ExecutionSequence`
    (:`then_0`
      ;[1 1 1] Forward drag system
      (if (`self.inHitbox`)
        (bind _asbp_seedboy (cast `/Game/FMP/Blueprints/BP_Seedboy` (`GameplayStatics.GetPlayerCharacter` 0)))
        (if (`/Game/FMP/Blueprints/BP_Seedboy.isDragging` _asbp_seedboy)
          (if (`/Game/FMP/Blueprints/BP_Seedboy.bisMovingRight` _asbp_seedboy)
            (`self.K2_AddActorLocalOffset` (* (80.0 0.0 0.0) _returnvalue))
            (else
              (`self.K2_AddActorLocalOffset` (* (-80.0 0.0 0.0) _returnvalue)))))))
    (:`then_1`
      ;[1 1 1] Drag opposite for left side
      (if (`self.leftOfBlock`)
        (bind _asbp_seedboy_2 (cast `/Game/FMP/Blueprints/BP_Seedboy` (`GameplayStatics.GetPlayerCharacter` 0)))
        (if (`/Game/FMP/Blueprints/BP_Seedboy.isDragging` _asbp_seedboy_2)
          (if (not (`/Game/FMP/Blueprints/BP_Seedboy.bisMovingRight` _asbp_seedboy_2))
            (`MovementComponent.StopMovementImmediately` (`Character.CharacterMovement` _asbp_seedboy_2))
            (`self.K2_AddActorLocalOffset` (* (-80.0 0.0 0.0) (`KismetMathLibrary.Conv_DoubleToVector` DeltaSeconds)))))
        (else
          ;[1 1 1] Drag opposite for right side
          (if (`self.rightOfBlock`)
            (bind _asbp_seedboy_3 (cast `/Game/FMP/Blueprints/BP_Seedboy` (`GameplayStatics.GetPlayerCharacter` 0)))
            (if (`/Game/FMP/Blueprints/BP_Seedboy.isDragging` _asbp_seedboy_3)
              (if (`/Game/FMP/Blueprints/BP_Seedboy.bisMovingRight` _asbp_seedboy_3)
                (`MovementComponent.StopMovementImmediately` (`Character.CharacterMovement` _asbp_seedboy_3))
                (`self.K2_AddActorLocalOffset` (* (80.0 0.0 0.0) (`KismetMathLibrary.Conv_DoubleToVector` DeltaSeconds)))))))))))

(fn `UserConstructionScript`)